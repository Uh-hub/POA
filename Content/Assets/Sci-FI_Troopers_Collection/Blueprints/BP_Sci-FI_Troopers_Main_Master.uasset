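; Base pawn for the Sci-Fi Troopers demo, letting the player cycle control between placed troopers.
; On BeginPlay each instance adds a demo widget to the viewport.
; Tab steps a wrapping index through all actors of this class, passes it to the next pawn, then blends the view and possesses it, carrying over control pitch and roll but not yaw.
; Escape quits the game.
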(event `self.ReceiveBeginPlay`
  (bind _returnvalue (`|CreateWidget` "/Game/Assets/Sci-FI_Troopers_Collection/DemoContent/W_DemoWidget.W_DemoWidget_C"))
  (`UserWidget.AddToViewport` _returnvalue 0))

(event `Key|Tab`
  (params (Key :type "Key Structure"))
  (bind _returnvalue (`GameplayStatics.GetPlayerController` 0))
  (bind _returnvalue_2 (`Controller.GetControlRotation` _returnvalue))
  (:`Pressed`
    (bind _outactors (`GameplayStatics.GetAllActorsOfClass` "BP_Sci-FI_Troopers_Main_Master_C"))
    (bind _output_get (set `self.Number` (+ (`self.Number`) 1)))
    (if (> _output_get (`KismetArrayLibrary.Array_LastIndex` _outactors))
      (set `self.Number` 0))
    (bind _outactors_2 (`GameplayStatics.GetAllActorsOfClass` "BP_Sci-FI_Troopers_Main_Master_C"))
    (bind _output (`|GetArrayItem` _outactors_2 (`self.Number`)))
    (set `/Game/Assets/Sci-FI_Troopers_Collection/Blueprints/BP_Sci-FI_Troopers_Main_Master.Number` (`self.Number`) _output)
    (`Controller.UnPossess` _returnvalue)
    (bind _output_get_2 (set `self.LastRotation` _returnvalue_2))
    (`PlayerController.SetViewTargetWithBlend` _returnvalue _output 0.5 "VTBlend_Cubic" 0.0 true)
    (`Controller.Possess` _returnvalue _output)
    (`Controller.SetControlRotation` _returnvalue (`KismetMathLibrary.MakeRotator` (.roll _output_get_2) (.pitch _output_get_2) (.yaw _returnvalue_2)))))

(event `Key|Escape`
  (params (Key :type "Key Structure"))
  (:`Pressed`
    (`KismetSystemLibrary.QuitGame` null "Quit")))

(fn `UserConstructionScript`)